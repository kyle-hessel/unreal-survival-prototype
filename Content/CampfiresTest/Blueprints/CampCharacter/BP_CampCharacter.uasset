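; BP_CampCharacter is the player character, extending C++ parent events for movement, sitting, lock-on, hit effects, building and inventory.
; Tick updates ABP_Explorer1 locomotion and scales walk and jump by exhaustion and speed multipliers, while Decelerate eases speed after sprinting.
; Opening inventory builds offset menus for backpack, pockets and active container under WBP_InventoryManager, raising braking friction at containers to prevent sliding.
; FindItemInInventory searches backpack, then pockets.
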(event `self.ReceiveBeginPlay`
  (bind _charactermovement (`self.CharacterMovement`))
  (`CampActionComponent.AddAction` (`self.ActionComp`) "/Game/CampfiresTest/Blueprints/Gameplay_Actions/BP_Action_Sprint.BP_Action_Sprint_C") ; Give our CampCharacter sprinting capabilities
  (set `self.DefaultJumpZVelocity` (`CharacterMovementComponent.JumpZVelocity` _charactermovement))
  (set `self.DefaultBrakingFriction` (`CharacterMovementComponent.BrakingFriction` _charactermovement))
  (bind _returnvalue (`|CreateWidget` "/Game/CampfiresTest/Blueprints/UI/WBP_CharacterStats.WBP_CharacterStats_C"))
  (`UserWidget.AddToViewport` _returnvalue 0))

(event `self.ReceiveTick`
  (params (DeltaSeconds :type "Float (single-precision)"))
  (bind _charactermovement (`self.CharacterMovement`))
  ;[0.5156 0.5156 0.5156] Update DetermineMovementState every frame so that LocomotionState is up to date. This also keeps our Locomotion state decoupled from our acceleration and deceleration; it only changes once it reaches certain speed thresholds.
  (`|ExecutionSequence`
    (:`then_0`
      (bind _asabp_explorer_1 (cast `/Game/CampfiresTest/Blueprints/CampCharacter/Animation/ABP_Explorer1` (`SkeletalMeshComponent.GetAnimInstance` (`self.Mesh`))))
      (`CampCharacterAnimInstance.UpdateAnimationProperties` _asabp_explorer_1)
      (`CampCharacterAnimInstance.DetermineMovementState` _asabp_explorer_1)
      ;[0.7917 0.7917 0.7917] Set our MaxWalkSpeed to the default set in the editor multiplied by our current ExhaustionMultiplier (and SpeedMultiplier from backpacks), but only when not running. When running let BP_Action_Sprint and Decelerate handle how to apply this value. Afterwards, set JumpZVelocity to be affected by modified versions of our exhaustion and speed multipliers if we are below the top energy tier or holding a backpack (no need to use DeltaTime here).
      (`|ExecutionSequence`
        (:`then_0`
          (if (not (`self.bSprinting`))
            (set `CharacterMovementComponent.MaxWalkSpeed` (* (`self.DefaultMaxWalkSpeed`) (`self.ExhaustionMultiplier`) (`self.SpeedMultiplier`)) _charactermovement)))
        (:`then_1`
          (bind _output_get (set `CharacterMovementComponent.JumpZVelocity` (* (`self.DefaultJumpZVelocity`) (`KismetMathLibrary.FClamp` (* (`self.ExhaustionMultiplier`) (`self.SpeedMultiplier`)) 0.5 3.0)) _charactermovement)))))))

(event `self.Decelerate`
  (params (DeltaTime :type "Float (single-precision)"))
  (bind _maxwalkspeed (`CharacterMovementComponent.MaxWalkSpeed` (`self.CharacterMovement`)))
  ;[0.1144 0.1202 0.2083] Decelerate each frame by a certain amount until we reach the amount we want to decelerate down to (when exiting out of sprint)
  (`parent.Decelerate` DeltaTime)
  (set `self.AdjustedDecelerationRate` (* (`self.DecelerationRate`) DeltaTime (`self.DeltaTimeScaleMultiplier_0`)))
  (if (not (`self.bIsAccelerating`))
    (set `CharacterMovementComponent.MaxWalkSpeed` (`KismetMathLibrary.Conv_IntToDouble` (`KismetMathLibrary.Round` (- _maxwalkspeed (`self.AdjustedDecelerationRate`)))) (`self.CharacterMovement`))
    (if (not (>= _maxwalkspeed (* (`self.DefaultMaxWalkSpeed`) (`self.SpeedMultiplier`) (`self.ExhaustionMultiplier`))))
      (set `self.bIsDecelerating` false)
      (set `self.bSprinting` false))
    (else
      (set `self.bIsDecelerating` false))))

(event `self.SitDown`
  ;[0.3854 0.1397 0.1282] Crank up Braking Friction when sitting so the player doesn't slide away from the sitting location.
  (`parent.SitDown`)
  (if (and (== (`self.bInCombat`) false) (== (`self.bLockedOnToEnemy`) false) (`KismetSystemLibrary.IsValid` (`CampInteractionComponent.GetCurrentSittingItem` (`self.InteractComp`))))
    (set `CharacterMovementComponent.BrakingFriction` 20.0 (`self.CharacterMovement`))))

(event `self.StandUp`
  ;[0.375 0.2338 0.1217] Reset Braking Friction when standing up so the player eases out of movement states again.
  (`parent.StandUp`)
  (set `CharacterMovementComponent.BrakingFriction` (`self.DefaultBrakingFriction`) (`self.CharacterMovement`)))

(event `self.LockOnToEnemy`
  (params (Enemy :type "CampEnemyBase Object Reference"))
  (`parent.LockOnToEnemy` Enemy)
  (set `CharacterMovementComponent.bOrientRotationToMovement` false (`self.CharacterMovement`)))

(event `self.ReleaseLockOn`
  (params (Enemy :type "CampEnemyBase Object Reference"))
  (`parent.ReleaseLockOn` Enemy)
  (set `CharacterMovementComponent.bOrientRotationToMovement` true (`self.CharacterMovement`)))

(event `self.PlayHitCameraShake`
  ;[0.2575 0.3087 1] Combat effects (camera shake, freeze-frames)
  (`GameplayStatics.PlayWorldCameraShake` "/Game/CampfiresTest/Blueprints/Animation/BP_CombatCameraShake.BP_CombatCameraShake_C" (`self.K2_GetActorLocation`) 0.0 (+ (`SpringArmComponent.TargetArmLength` (`self.CameraBoom`)) 100.0) 1.0 true))

(event `self.PlayHitFreezeFrame`
  (params (FreezeFrameTimer :type "Float (single-precision)") (TimeDilationFactor :type "Float (single-precision)"))
  ;[0.2575 0.3087 1] Combat effects (camera shake, freeze-frames)
  (`GameplayStatics.SetGlobalTimeDilation` TimeDilationFactor)
  (`KismetSystemLibrary.K2_SetTimerDelegate` (delegate `UnFreezeFrame`) (* TimeDilationFactor FreezeFrameTimer)))

(event `UnFreezeFrame`
  ;[0.2575 0.3087 1] Combat effects (camera shake, freeze-frames)
  (`GameplayStatics.SetGlobalTimeDilation` 1.0))

(event `self.ToggleBuildMenu`
  ;[0.5521 0.5521 0.5521] Create build menu.
  (if (not (`self.bInBuildMenu`))
    (bind _returnvalue (`|CreateWidget` "/Game/CampfiresTest/Blueprints/UI/Building/WBP_BuildMenu.WBP_BuildMenu_C" (cast `PlayerController` (`self.GetController`) :!pure true) self))
    (`UserWidget.AddToPlayerScreen` _returnvalue 0)))

(event `InputAction|Inventory`
  (params (Key :type "Key Structure"))
  ;[0.09896 0.09896 0.09896 0.5] Inventory-related code
  ;;[0.2303 0.349 0.2108] When Inventory key is pressed, determine if it was on a gamepad or keyboard and then call event Open Inventory.
  (:`Pressed`
    (if (not (`self.bInBuildMenu`))
      (if (`KismetInputLibrary.Key_IsGamepadKey` Key)
        (set `self.bOpenInventoryWithGamepad` true)
        (else
          (set `self.bOpenInventoryWithGamepad` false)))
      (`self.OpenInventory`))))

(event `self.OpenInventory`
  (bind _openinventories (`self.OpenInventories`))
  (bind _bopeninventorywithgamepad (`self.bOpenInventoryWithGamepad`))
  (bind _bsortbystack (`self.bSortByStack`))
  (bind _activecontainerobject (`self.ActiveContainerObject`))
  (bind _openinventories_2 (`self.OpenInventories`))
  (bind _asplayer_controller (cast `PlayerController` (`self.GetController`) :!pure true))
  (bind _heldbackpack (`CampInteractionComponent.HeldBackpack` (`self.InteractComp`)))
  (bind _returnvalue_x (`KismetMathLibrary.BreakVector2D` (`SlateBlueprintLibrary.GetAbsoluteSize` (`Widget.GetCachedGeometry` (`|GetArrayItem` (`self.OpenInventoryMenus`))))))
  ;[0.09896 0.09896 0.09896 0.5] Inventory-related code
  ;;[0.1266 0.04736 0.1979] Opens inventory or inventories depending on if a backpack is being worn and if a storage object is being accessed. Also sets bIsOpen back to false if the inventory is already opened when this key is pressed, but the inventory itself is removed in WBP_InventoryMenu from the same trigger.
  (`parent.OpenInventory`)
  (if (== (`CampInventoryComponent.bIsOpen` (`self.InventoryComp`)) true)
    (for _array_element (`self.OpenInventories`)
      (set `CampInventoryComponent.bIsOpen` false _array_element))
    (`KismetArrayLibrary.Array_Clear` (`self.OpenInventories`))
    (`KismetArrayLibrary.Array_Clear` (`self.OpenInventoryMenus`))
    (`/Engine/EditorBlueprintResources/StandardMacros.IsValid` (`self.ActiveContainerObject`)
      (:`Is Valid`
        (set `CharacterMovementComponent.BrakingFriction` (`self.DefaultBrakingFriction`) (`self.CharacterMovement`))))
    (else
      (`|ExecutionSequence`
        (:`then_0`
          (`/Engine/EditorBlueprintResources/StandardMacros.IsValid` _heldbackpack
            (:`Is Valid`
              (`/Engine/EditorBlueprintResources/StandardMacros.IsValid` _activecontainerobject
                (:`Is Valid`
                  (`KismetArrayLibrary.Array_Add` (`self.OpenInventories`) (`CampBackpack.InventoryComp` (`CampInteractionComponent.HeldBackpack` (`self.InteractComp`))))
                  (`KismetArrayLibrary.Array_Add` (`self.OpenInventories`) (`self.InventoryComp`))
                  (`KismetArrayLibrary.Array_Add` (`self.OpenInventories`) (`self.ActiveContainerInventoryComp`)))
                (:`Is Not Valid`
                  (`KismetArrayLibrary.Array_Add` _openinventories (`CampBackpack.InventoryComp` _heldbackpack))
                  (`KismetArrayLibrary.Array_Add` _openinventories (`self.InventoryComp`)))))
            (:`Is Not Valid`
              (`/Engine/EditorBlueprintResources/StandardMacros.IsValid` _activecontainerobject
                (:`Is Valid`
                  (`KismetArrayLibrary.Array_Add` _openinventories_2 (`self.InventoryComp`))
                  (`KismetArrayLibrary.Array_Add` _openinventories_2 (`self.ActiveContainerInventoryComp`)))
                (:`Is Not Valid`
                  (`KismetArrayLibrary.Array_Add` (`self.OpenInventories`) (`self.InventoryComp`)))))))
        (:`then_1`
          (for (_array_element_2 _array_index) (`self.OpenInventories`)
            (set `CampInventoryComponent.bIsOpen` true _array_element_2)
            (if (== _array_index 0)
              (bind _returnvalue (`KismetStringLibrary.Conv_StringToName` (`CampInventoryComponent.InventoryName` _array_element_2)))
              (bind _returnvalue_2 (`|CreateWidget` "/Game/CampfiresTest/Blueprints/UI/WBP_InventoryMenu.WBP_InventoryMenu_C" _asplayer_controller _returnvalue _array_element_2 _bopeninventorywithgamepad true _bsortbystack))
              (`UserWidget.AddToPlayerScreen` _returnvalue_2 0)
              (`KismetArrayLibrary.Array_Add` (`self.OpenInventoryMenus`) _returnvalue_2)
              (else
                (bind _returnvalue_3 (`|CreateWidget` "/Game/CampfiresTest/Blueprints/UI/WBP_InventoryMenu.WBP_InventoryMenu_C" _asplayer_controller _returnvalue _array_element_2 _bopeninventorywithgamepad false _bsortbystack))
                (`UserWidget.AddToPlayerScreen` _returnvalue_3 0)
                (`KismetArrayLibrary.Array_Add` (`self.OpenInventoryMenus`) _returnvalue_3))))
          (for (_array_element_3 _array_index_2) (`self.OpenInventoryMenus`)
            (if (> _array_index_2 0)
              (`UserWidget.SetPositionInViewport` _array_element_3 (`KismetMathLibrary.MakeVector2D` (* (+ _returnvalue_x (`self.InventoryOffset`)) (`WidgetLayoutLibrary.GetViewportScale`))) true)
              (set `self.InventoryOffset` (+ (`self.InventoryOffset`) 600.0))
              (else
                (set `self.InventoryOffset` 600.0))))
          (bind _returnvalue_4 (`|CreateWidget` "/Game/CampfiresTest/Blueprints/UI/WBP_InventoryManager.WBP_InventoryManager_C" null (`self.OpenInventoryMenus`) self (`self.bOpenInventoryWithGamepad`)))
          (`UserWidget.AddToPlayerScreen` _returnvalue_4 0)
          (`/Engine/EditorBlueprintResources/StandardMacros.IsValid` (`self.ActiveContainerObject`)
            (:`Is Valid`
              (set `CharacterMovementComponent.BrakingFriction` 20.0 (`self.CharacterMovement`)) ; Avoids the player sliding out of the overlap box for the trunk while its inventory is open and breaking a lot of things :^)
            )))))))

(event `self.InventoryComp.OnItemPickup`
  ;[0.09896 0.09896 0.09896 0.5] Inventory-related code
  ;;[0.3021 0.1889 0.1479] Refresh open inventories if an item is added (There might be some redundant refreshes happening because of this).
  (for _array_element (`self.OpenInventoryMenus`)
    (`/Game/CampfiresTest/Blueprints/UI/WBP_InventoryMenu.RefreshInventory` _array_element)))

(event `CloseOpenInventories`
  ;[0.09896 0.09896 0.09896 0.5] Inventory-related code
  (for _array_element (`self.OpenInventoryMenus`)
    (`/Game/CampfiresTest/Blueprints/UI/WBP_InventoryMenu.CloseInventory` _array_element))
  (`self.OpenInventory`))

(fn `FindItemInInventory`
  (params (ItemName :type Name) (Quantity :type Integer))
  (returns (ItemNameAndNumber :type Name) (ItemFound :type Boolean) (InBackpack :type Boolean))
  (bind _heldbackpack (`CampInteractionComponent.HeldBackpack` (`self.InteractComp`)))
  (bind _inventorycontents (`CampInventoryComponent.InventoryContents` (`self.InventoryComp`)))
  (bind _inventorycontents_2 (`CampInventoryComponent.InventoryContents` (`CampBackpack.InventoryComp` _heldbackpack)))
  (`/Engine/EditorBlueprintResources/StandardMacros.IsValid` _heldbackpack ; If there's a backpack, search that first. If not, jump straight to pockets.
    (:`Is Valid`
      (bind _keys (`BlueprintMapLibrary.Map_Keys` _inventorycontents_2))
      (for _array_element _keys
        (bind _outstring (`/Game/CampfiresTest/Blueprints/Core/BP_CampHelperFunctions.RemoveNumbersFromString` (`KismetStringLibrary.Conv_NameToString` _array_element)))
        (if (and (== ItemName (`KismetStringLibrary.Conv_StringToName` _outstring)) (>= (`BlueprintMapLibrary.Map_Find` _inventorycontents_2 _array_element) Quantity))
          (`KismetSystemLibrary.PrintString` "ITEM FOUND" false)
          (return _array_element true true))))
    (:`Is Not Valid`
      _))
  (bind _keys_2 (`BlueprintMapLibrary.Map_Keys` _inventorycontents)) ; Search pockets (either first or if backpack came back empty).
  (for _array_element_2 _keys_2
    (bind _outstring_2 (`/Game/CampfiresTest/Blueprints/Core/BP_CampHelperFunctions.RemoveNumbersFromString` (`KismetStringLibrary.Conv_NameToString` _array_element_2)))
    (if (and (== ItemName (`KismetStringLibrary.Conv_StringToName` _outstring_2)) (>= (`BlueprintMapLibrary.Map_Find` _inventorycontents _array_element_2) Quantity))
      (`KismetSystemLibrary.PrintString` "ITEM FOUND" false)
      (return _array_element_2 true false)))
  (return "None" false false) ; If loop(s) completed without finding the item, return None.
)

(fn `UserConstructionScript`)