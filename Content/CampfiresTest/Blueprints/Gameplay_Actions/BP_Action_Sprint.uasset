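; Sprint action that ramps a CampCharacter's MaxWalkSpeed up to a top sprint speed.
; On start it derives acceleration and top speed from the character's speed multiplier, exhaustion and sprint bonus.
; Each tick it adds delta-scaled acceleration, pausing while the anim blueprint reports Jump and flagging deceleration if exhaustion multiplier drops.
; On stop it sets the deceleration rate and flag, leaving the slowdown to CampCharacter.
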(event `self.StartAction`
  (params (Instigator :type "Actor Object Reference"))
  ;[1 0.4148 0.2645] Set our TopSprintSpeed based on our CampCharacter movement component's MaxWalkSpeed (fetched from its CharacterMovementComponent in BeginPlay) plus SprintBonus.
  (`parent.StartAction` Instigator)
  (bind _ascamp_character (cast `CampCharacter` Instigator))
  (bind _speedmultiplier (`CampCharacter.SpeedMultiplier` _ascamp_character))
  (set `self.AccelerationRate` (* (`CampCharacter.AccelerationRate` _ascamp_character) _speedmultiplier)) ; Set our local acceleration rate variable equal to CampCharacter's
  (bind _exhaustionmultiplier (`CampCharacter.ExhaustionMultiplier` _ascamp_character))
  (set `self.TopSprintSpeed` (* _speedmultiplier (+ (* (`CampCharacter.DefaultMaxWalkSpeed` _ascamp_character) _exhaustionmultiplier) (* _exhaustionmultiplier (`self.SprintBonus`)))))
  (set `self.CachedExhaustionMultiplier` _exhaustionmultiplier)
  (bind _asabp_camp_character (cast `/Game/CampfiresTest/Blueprints/CampCharacter/Animation/ABP_CampCharacter` (`SkeletalMeshComponent.GetAnimInstance` (`Character.Mesh` _ascamp_character))))
  (set `self.bIsInAir` (`|EnumEquality` (`CampCharacterAnimInstance.LocomotionState` _asabp_camp_character) "LOCO_Jump")))

(event `self.TickAction`
  (params (Instigator :type "Actor Object Reference") (DeltaTime :type "Float (single-precision)"))
  (bind _returnvalue (`Actor.GetComponentByClass` Instigator "/Script/Engine.CharacterMovementComponent"))
  ;[0.4667 0.2339 1] (Acceleration) Increment CharacterMovementComponent's MaxWalkSpeed every frame until it is equal to the TopSprintSpeed we set in our StartAction implementation above.
  (`parent.TickAction` Instigator DeltaTime)
  (set `self.AdjustedAccelerationRate` (* (`self.AccelerationRate`) DeltaTime (`self.DeltaTimeScaleMultiplier`))) ; Account for DeltaTime
  (if (not (`self.bIsInAir`))
    (bind _ascamp_character (cast `CampCharacter` Instigator))
    (if (< (`CampCharacter.ExhaustionMultiplier` _ascamp_character) (`self.CachedExhaustionMultiplier`))
      (set `CampCharacter.bIsAccelerating` false _ascamp_character) ; Decelerate back to walking if we drop an energy tier while running.
      (set `CampCharacter.bIsDecelerating` true _ascamp_character)
      (else
        (set `CampCharacter.bIsAccelerating` true _ascamp_character)
        (if (<= (+ (`CharacterMovementComponent.MaxWalkSpeed` _returnvalue) (`self.AdjustedAccelerationRate`)) (`self.TopSprintSpeed`))
          (set `CharacterMovementComponent.MaxWalkSpeed` (`KismetMathLibrary.Conv_IntToDouble` (`KismetMathLibrary.Round` (+ (`CharacterMovementComponent.MaxWalkSpeed` _returnvalue) (`self.AdjustedAccelerationRate`)))) _returnvalue))))
    (else
      (bind _ascamp_character_2 (cast `CampCharacter` Instigator)) ; If we are jumping, keep checking if we stop jumping while ticking\nso that if we land we start accelerating again.
      (bind _asabp_camp_character (cast `/Game/CampfiresTest/Blueprints/CampCharacter/Animation/ABP_CampCharacter` (`SkeletalMeshComponent.GetAnimInstance` (`Character.Mesh` _ascamp_character_2))))
      (set `self.bIsInAir` (`|EnumEquality` (`CampCharacterAnimInstance.LocomotionState` _asabp_camp_character) "LOCO_Jump")))))

(event `self.StopAction`
  (params (Instigator :type "Actor Object Reference"))
  ;[0.3353 0.3596 1] If we stop our sprint action, set decelerating to true and let CampCharacter determine how much to decelerate (to walking, to standstill, etc)
  (`parent.StopAction` Instigator)
  (bind _ascamp_character (cast `CampCharacter` Instigator))
  (set `CampCharacter.bIsAccelerating` false _ascamp_character)
  (set `CampCharacter.DecelerationRate` (* (`CampCharacter.DefaultDecelerationRate` _ascamp_character) (`CampCharacter.SpeedMultiplier` _ascamp_character)) _ascamp_character)
  (set `CampCharacter.bIsDecelerating` true _ascamp_character))