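; Interactable camp backpack that changes the player's walk speed while equipped, intended as a slowdown, extending equip and drop logic from its parent class.
; Interacting multiplies the character's SpeedMultiplier by the backpack's modifier and recalculates max walk speed from default speed and exhaustion.
; A successful drop resets the multiplier and speed.
; Both paths stop the Sprint action to work around stale values in BP_Action_Sprint.
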(event `CampInteractionInterface.Interact`
  (params (InstigatorPawn :type "Pawn Object Reference"))
  ;[0.6042 0.6042 0.6042] Equip backpack: implemented in C++
  (`parent.Interact` InstigatorPawn)
  ;[0.2083 0.2083 0.2083] Extra functionality: add speed multiplier to our player when equipping the bag and multiply it by the player's speed, which will slow the player in this case.
  (bind _ascamp_character (cast `CampCharacter` InstigatorPawn))
  (bind _output_get (set `CampCharacter.SpeedMultiplier` (* (`CampCharacter.SpeedMultiplier` _ascamp_character) (`self.BackpackSpeedModifier`)) _ascamp_character))
  (set `CharacterMovementComponent.MaxWalkSpeed` (* (* (`CampCharacter.DefaultMaxWalkSpeed` _ascamp_character) (`CampCharacter.ExhaustionMultiplier` _ascamp_character)) _output_get) (cast `CharacterMovementComponent` (`Pawn.GetMovementComponent` _ascamp_character) :!pure true))
  (bind _actioncomp (`CampCharacter.ActionComp` _ascamp_character))
  ;[0.07292 0.07292 0.07292] Stop our sprint to revert back to walking, avoiding a bug that stops relevant values in BP_Action_Sprint from being updated.
  (for _array_element (`CampActionComponent.Actions` _actioncomp)
    (bind _actionname (`CampAction.ActionName` _array_element))
    (if (== _actionname "Sprint")
      (`CampActionComponent.StopActionByName` _actioncomp null _actionname))))

(fn `DropBackpack`
  (returns (ReturnValue :type Boolean))
  (bind _campcharacter (`self.CampCharacter`))
  (bind _actioncomp (`CampCharacter.ActionComp` _campcharacter))
  (bind _returnvalue (`parent.DropBackpack`))
  (if _returnvalue
    ;[0.5312 0.5312 0.5312] Reset the player's speed values.
    (set `CharacterMovementComponent.MaxWalkSpeed` (* (`CampCharacter.DefaultMaxWalkSpeed` _campcharacter) (`CampCharacter.ExhaustionMultiplier` _campcharacter)) (cast `CharacterMovementComponent` (`Pawn.GetMovementComponent` _campcharacter) :!pure true))
    (set `CampCharacter.SpeedMultiplier` 1.0 _campcharacter)
    ;[0.07292 0.07292 0.07292] Stop our sprint to revert back to walking, avoiding a bug that stops relevant values in BP_Action_Sprint from being updated.
    (for _array_element (`CampActionComponent.Actions` _actioncomp)
      (bind _actionname (`CampAction.ActionName` _array_element))
      (if (== _actionname "Sprint")
        (`CampActionComponent.StopActionByName` _actioncomp null _actionname)
        (return _returnvalue)))))

(fn `UserConstructionScript`)